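; Wave controller actor that spawns groups of AI enemies around itself, starting the first wave on BeginPlay.
; SpawnWave runs a looping one-second delay countdown, then increments the wave index and spawns twice that many enemies, capped at ten, at random navigable points.
; Each enemy gets a reference to the controller and raises EnemyCount; an event lowers the count, but nothing here triggers the next wave.
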(event Custom|SpawnWave
  (Variables|Default|Settimer 5.0)
  (Utilities|FlowControl|Delay 1.0 :!label _label)
  (bind _result (Math|Float|DecrementFloat (Variables|Default|Gettimer))
    (:%20%20
      (bind _output_get (Variables|Default|Settimer _result))
      (if (<= _output_get 0.0)
        (bind _result_2 (Math|Integer|IncrementInt (Variables|Default|GetwaveIndex))
          (:%20%20
            (bind _output_get_2 (Variables|Default|SetwaveIndex _result_2))
            (if (<= (* _output_get_2 2) 10)
              (for _index (range 1 (* _output_get_2 2))
                (bind _returnvalue (AI|SpawnAIFromClass "/Game/Blueprints/Enemies/Enemy.Enemy_C" 0 (.RandomLocation (Class|NavigationSystemV1|GetRandomPointinNavigableRadius (Transformation|GetActorLocation) 2.5e+03 0 0)) "0, 0, 0" false))
                (bind _asenemy (Utilities|Casting|CastToEnemy _returnvalue))
                (Variables|/Game/Blueprints/Enemies/Enemy.Enemy_C|SetwaveContrRef _asenemy self)
                (bind _result_3 (Math|Integer|IncrementInt (Variables|Default|GetenemyCount))
                  (:%20%20
                    (Variables|Default|SetenemyCount _result_3))))
              (else
                (for _index_2 (range 1 10)
                  (bind _returnvalue_2 (AI|SpawnAIFromClass "/Game/Blueprints/Enemies/Enemy.Enemy_C" 0 (.RandomLocation (Class|NavigationSystemV1|GetRandomPointinNavigableRadius (Transformation|GetActorLocation) 2.5e+03 0 0)) "0, 0, 0" false))
                  (bind _asenemy_2 (Utilities|Casting|CastToEnemy _returnvalue_2))
                  (Variables|/Game/Blueprints/Enemies/Enemy.Enemy_C|SetwaveContrRef _asenemy_2 self)
                  (bind _result_4 (Math|Integer|IncrementInt (Variables|Default|GetenemyCount))
                    (:%20%20
                      (Variables|Default|SetenemyCount _result_4))))))))
        (else
          (goto _label))))))

(event Custom|EnemyCount--
  (bind _result (Math|Integer|DecrementInt (Variables|Default|GetenemyCount))
    (:%20%20
      (Variables|Default|SetenemyCount _result))))

(event EventBeginPlay
  (CallFunction|SpawnWave))

(fn ConstructionScript)