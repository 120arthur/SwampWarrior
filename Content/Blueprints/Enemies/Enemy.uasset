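; Wave-based enemy character that patrols random navmesh points, chases and attacks a nearby living player, and can drop power-ups.
; BeginPlay attaches damage volumes to both hand sockets.
; Tick drives AIMoveTo and briefly raises an attack flag on arrival.
; Damage pauses attacks or, when lethal, sets a death flag and updates the wave controller; DestroySelf randomly spawns a speed, defense or attack boost before destroying the actor.
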(event Custom|TakeDamage
  (params (damage :type Float%20%28single-precision%29))
  (bind _wavecontrref (Variables|Default|GetwaveContrRef))
  ;[1 1 1] Take Damage
  (if (and (not (Variables|Default|GetisTakingDamage)) (not (<= (Variables|Default|GethealthPoints) 0.0)))
    (Variables|Default|SetisTakingDamage true)
    (Variables|Default|SethealthPoints (- (Variables|Default|GethealthPoints) damage))
    (Variables|Default|SetcanAttack false)
    (if (<= (Variables|Default|GethealthPoints) 0.0)
      ;[1 1 1] Death + Spawn Power Up
      ;;[1 1 1] Update Wave Controller
      (Default|EnemyCount-- _wavecontrref)
      (if (<= (Variables|/Game/Blueprints/Enemies/WaveeController.WaveeController_C|GetenemyCount _wavecontrref) 0)
        (Default|SpawnWave (Variables|Default|GetwaveContrRef)))
      (Variables|Default|SetshouldDie true)
      (else
        (Utilities|FlowControl|Delay 2.0)
        (Variables|Default|SetcanAttack true)))))

(event Custom|DestroySelf
  (bind _rootcomponent (Variables|Transformation|GetRootComponent))
  (bind _relativelocation (Variables|/Script/Engine.SceneComponent|GetRelativeLocation _rootcomponent))
  (bind _returnvalue (Math|Conversions|ToTransform(Vector) _relativelocation))
  ;[1 1 1] Death + Spawn Power Up
  (if (== (Math|Random|RandomIntegerinRange 0 3) 2)
    (switch int (Math|Random|RandomIntegerinRange 0 2)
      (:Default
        (Game|SpawnActorfromClass "/Game/Blueprints/PowerUps/BP_SpeedUp.BP_SpeedUp_C" _returnvalue "Undefined" 0 0 :!label _label))
      (:0
        (Game|SpawnActorfromClass "/Game/Blueprints/PowerUps/BP_DefenseUp.BP_DefenseUp_C" _returnvalue "Undefined" 0 0))
      (:1
        (Game|SpawnActorfromClass "/Game/Blueprints/PowerUps/BP_AttackUp.BP_AttackUp_C" _returnvalue "Undefined" 0 0))
      (:2
        (goto _label))))
  (Actor|DestroyActor))

(event EventTick
  (params (DeltaSeconds :type Float%20%28single-precision%29))
  (bind _returnvalue (Game|Player|GetPlayerPawn 0))
  (bind _self self)
  ;[1 1 1] AI
  (if (and (<= (Math|Vector|Distance(Vector) (Transformation|GetActorLocation self) (Transformation|GetActorLocation _returnvalue)) 1e+03) (not (Variables|Default|GetshouldDie)))
    ;;[1 1 1] Follow Player
    (bind _asmain_pawn__sw (Utilities|Casting|CastToMainPawn-SW _returnvalue))
    (if (not (Variables|/Game/Blueprints/Player/MainPawn-SW.MainPawn-SW_C|GetshouldDie _asmain_pawn__sw))
      (AI|AIMoveTo _self "0, 0, 0" _returnvalue 1.5e+02 false
        (:OnSuccess
          ;;[1 1 1] Attack Player
          (if (not (Variables|Default|GetisTakingDamage))
            (if (Variables|Default|GetcanAttack)
              (Variables|/Script/Engine.CharacterMovementComponent|SetMaxWalkSpeed (Variables|Character|GetCharacterMovement) 1.5e+02)
              (Variables|Default|SetshouldAttack true)
              (Utilities|FlowControl|Delay 0.2)
              (Variables|Default|SetshouldAttack false)
              (Variables|/Script/Engine.CharacterMovementComponent|SetMaxWalkSpeed (Variables|Character|GetCharacterMovement) 4e+02))))))
    (else
      ;[1 1 1] Patroling
      (if (not (Variables|Default|GetisPatrolling))
        (bind _randomlocation (Class|NavigationSystemV1|GetRandomLocationinNavigableRadius (Transformation|GetActorLocation) 1.5e+03 0 0))
        (AI|AIMoveTo _self _randomlocation 0 2e+02 false
          (:then
            (Variables|Default|SetisPatrolling true))
          (:OnSuccess
            (Variables|Default|SetisPatrolling false)))))))

(event EventBeginPlay
  ;[1 1 1] Attach DamageVolume to Hands
  (bind _returnvalue (Game|SpawnActorfromClass "/Game/Blueprints/Enemies/EnemyDamageVol.EnemyDamageVol_C" (Transformation|GetSocketTransform (Variables|Character|GetMesh) "RightHandSocket" "RTS_World") "Undefined" 0 0))
  (bind _output_get (Variables|Default|SetdamageVolumeR _returnvalue))
  (Transformation|AttachComponentToComponent _output_get (Variables|Character|GetMesh) "RightHandSocket" "SnapToTarget" "SnapToTarget" "SnapToTarget" true)
  (bind _returnvalue_2 (Game|SpawnActorfromClass "/Game/Blueprints/Enemies/EnemyDamageVol.EnemyDamageVol_C" (Transformation|GetSocketTransform (Variables|Character|GetMesh) "LeftHandSocket" "RTS_World") "Undefined" 0 0))
  (bind _output_get_2 (Variables|Default|SetdamageVolumeL _returnvalue_2))
  (Transformation|AttachComponentToComponent _output_get_2 (Variables|Character|GetMesh) "LeftHandSocket" "SnapToTarget" "SnapToTarget" "SnapToTarget" true))

(fn ConstructionScript)