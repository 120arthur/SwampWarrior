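; Calango enemy Blueprint that arms both hands of its mesh with damage volumes.
; On BeginPlay it spawns an EnemyDamageVol actor at the right and left hand sockets, stores each reference, and snaps it to its socket so it follows the skeleton.
; The construction script only calls the parent's, and this graph holds no other logic.
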(event EventBeginPlay
  ;[1 1 1] Attach DamageVolume to Hands
  (bind _returnvalue (Game|SpawnActorfromClass "/Game/Blueprints/Enemies/EnemyDamageVol.EnemyDamageVol_C" (Transformation|GetSocketTransform (Variables|Character|GetMesh) "RightHandSocket" "RTS_World") "Undefined" 0 0))
  (bind _output_get (Variables|Default|SetdamageVolumeR _returnvalue))
  (Transformation|AttachComponentToComponent _output_get (Variables|Character|GetMesh) "RightHandSocket" "SnapToTarget" "SnapToTarget" "SnapToTarget" true)
  (bind _returnvalue_2 (Game|SpawnActorfromClass "/Game/Blueprints/Enemies/EnemyDamageVol.EnemyDamageVol_C" (Transformation|GetSocketTransform (Variables|Character|GetMesh) "LeftHandSocket" "RTS_World") "Undefined" 0 0))
  (bind _output_get_2 (Variables|Default|SetdamageVolumeL _returnvalue_2))
  (Transformation|AttachComponentToComponent _output_get_2 (Variables|Character|GetMesh) "LeftHandSocket" "SnapToTarget" "SnapToTarget" "SnapToTarget" true))

(fn ConstructionScript
  (|CallParentFunction))