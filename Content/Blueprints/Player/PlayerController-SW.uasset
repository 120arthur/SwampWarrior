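; Player controller that routes action inputs to the player's MainPawn-SW and opens the pause menu.
; On BeginPlay it casts player pawn 0 to MainPawn-SW and caches the reference.
; Recover HP, Dodge, Melee Attack and Transform presses call the matching functions on that pawn.
; The Pause press creates a PauseMenu widget and adds it to the viewport, without setting game pause here.
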(event EventBeginPlay
  ;[1 1 1] Set ControlledPawn Ref
  (bind _asmain_pawn__sw (Utilities|Casting|CastToMainPawn-SW (Game|Player|GetPlayerPawn 0)))
  (Variables|Default|SetmyMainPawn _asmain_pawn__sw))

(event Input|ActionEvents|InputActionPause
  (params (Key :type Key%20Structure :default "None"))
  ;[1 1 1] Pause Game
  (:Pressed
    (bind _returnvalue (UserInterface|CreateWidget "/Game/Blueprints/UI/PauseMenu.PauseMenu_C"))
    (UserInterface|Viewport|AddtoViewport _returnvalue 0)))

(event Input|ActionEvents|InputActionMeleeAttack
  (params (Key :type Key%20Structure :default "None"))
  ;[1 1 1] Melee Attack Input
  (:Pressed
    (Default|MeleeAttack (Variables|Default|GetmyMainPawn))))

(event Input|ActionEvents|InputActionRangedAttack
  (params (Key :type Key%20Structure :default "None")))

(event Input|ActionEvents|InputActionRecoverHP
  (params (Key :type Key%20Structure :default "None"))
  ;[1 1 1] Recover HP Input
  (:Pressed
    (Default|RecoverHP (Variables|Default|GetmyMainPawn))))

(event Input|ActionEvents|InputActionTransform
  (params (Key :type Key%20Structure :default "None"))
  ;[1 1 1] Transform Input
  (:Pressed
    (Default|Transform (Variables|Default|GetmyMainPawn))))

(event Input|ActionEvents|InputActionDodge
  (params (Key :type Key%20Structure :default "None"))
  ;[1 1 1] Dodge
  (:Pressed
    (Default|Dodge (Variables|Default|GetmyMainPawn))))

(fn ConstructionScript)